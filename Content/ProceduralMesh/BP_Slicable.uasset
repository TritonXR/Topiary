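; BP_Slicable is an actor whose mesh can be cut in two along an arbitrary plane at runtime.
; Its construction script copies an assigned static mesh into a procedural mesh with collision, then destroys the static mesh component.
; SliceMe cuts the given procedural mesh, caps it with pine wood material, enables physics on the new half and fires a radial force impulse at the cut.
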(event `SliceMe`
  (params (ProcComp :type "ProceduralMeshComponent Object Reference") (Location :type "Vector Structure") (Normal :type "Vector Structure"))
  (bind _radialforce (`self.RadialForce`))
  (bind _outotherhalfprocmesh (`KismetProceduralMeshLibrary.SliceProceduralMesh` ProcComp Location Normal true "CreateNewSectionForCap" "/Game/StarterContent/Materials/M_Wood_Pine.M_Wood_Pine"))
  (`PrimitiveComponent.SetSimulatePhysics` _outotherhalfprocmesh true)
  (`PrimitiveComponent.SetCollisionObjectType` _outotherhalfprocmesh "ECC_GameTraceChannel1")
  (`SceneComponent.K2_SetWorldLocation` _radialforce Location false true)
  (`RadialForceComponent.FireImpulse` _radialforce))

(event `self.ReceiveBeginPlay`)

(fn `UserConstructionScript`
  (`StaticMeshComponent.SetStaticMesh` (`self.StaticMesh`) (`self.StaticMeshToCopy`))
  (`KismetProceduralMeshLibrary.CopyProceduralMeshFromStaticMeshComponent` (`self.StaticMesh`) 0 (`self.ProceduralMesh`) true)
  (`ActorComponent.K2_DestroyComponent` (`self.StaticMesh`)))