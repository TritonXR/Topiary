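; BP_BushToSlice is a bush actor prepared for runtime mesh slicing.
; Its construction script copies the MeshToSlice static mesh into a ProceduralMesh component with collision and tags the actor Slicable.
; Pickup and Drop events are empty stubs; their physics toggle and attach/detach logic is disconnected, with a note that picking up and interacting with sliced meshes fail.
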(event `/Game/VirtualRealityBP/Blueprints/PickupActorInterface.Pickup`
  (params (AttachTo :type "SceneComponent Object Reference"))
  ;[1 1 1] Picking up doesn't work + same problem with interacting with sliced proc meshes (like the old)
)

(event `/Game/VirtualRealityBP/Blueprints/PickupActorInterface.Drop`
  ;[1 1 1] Picking up doesn't work + same problem with interacting with sliced proc meshes (like the old)
)

(fn `UserConstructionScript`
  (`KismetProceduralMeshLibrary.CopyProceduralMeshFromStaticMeshComponent` (`self.MeshToSlice`) 0 (`self.ProceduralMesh`) true)
  (set `self.Tags` (`|MakeArray` "Slicable" :!type "Name")))